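; Twitter integration Blueprint that attempts the first OAuth step, requesting a request token on BeginPlay.
; It POSTs a VaRest JSON request with a random Base64 nonce, out-of-band callback and hardcoded consumer key as separate headers, without a signature.
; Completion prints headers and response JSON in green; failure prints the header count in red.
; The Twitter widget creation and Authorization header nodes are unconnected, and no token is stored.
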(event `self.ReceiveBeginPlay`
  (bind _oauthreqtoken (`self.OAuthReqToken`))
  (bind _output_get (set `self.OAuthReqToken` (`VaRestRequestJSON.ConstructRequestExt` "POST" "json")))
  (bind _returnvalue (`VaRestLibrary.Base64Encode` (`KismetStringLibrary.Concat_StrStr` (`KismetStringLibrary.Conv_IntToString` (`KismetMathLibrary.RandomIntegerInRange` 10000 99999)) "qwertyuiopasdfghjklzxcvbnm0")))
  (`VaRestRequestJSON.SetHeader` _output_get "oauth_nonce=" _returnvalue)
  (`VaRestRequestJSON.SetHeader` _output_get "oauth_callback" "oob")
  (`VaRestRequestJSON.SetHeader` _output_get "oauth_consumer_key" "QWBcTJZseiAICZiA4D9ifrFzp")
  (add `VaRestRequestJSON.OnRequestComplete` _oauthreqtoken (delegate `OAuthReqTokenComplete`))
  (add `VaRestRequestJSON.OnRequestFail` _oauthreqtoken (delegate `OAuthReqTokenFail`))
  (`VaRestRequestJSON.ProcessURL` (`self.OAuthReqToken`) "https://api.twitter.com/oauth/request_token"))

(event `OAuthReqTokenComplete`
  (params (Request :type "VaRestRequestJSON Object Reference"))
  (bind _returnvalue (`VaRestRequestJSON.GetAllResponseHeaders` Request))
  (for _array_element _returnvalue
    (`KismetSystemLibrary.PrintString` _array_element true true (struct :`R` 0.101521 :`G` 1.0 :`A` 1.0) 15.0))
  (bind _returnvalue_2 (`VaRestRequestJSON.GetResponseObject` Request))
  (`KismetSystemLibrary.PrintString` (`VaRestJsonObject.EncodeJsonToSingleString` _returnvalue_2) true true (struct :`R` 0.101521 :`G` 1.0 :`A` 1.0) 15.0))

(event `OAuthReqTokenFail`
  (params (Request :type "VaRestRequestJSON Object Reference"))
  (bind _returnvalue (`VaRestRequestJSON.GetAllResponseHeaders` Request))
  (`KismetSystemLibrary.PrintString` (`KismetStringLibrary.Conv_IntToString` (`KismetArrayLibrary.Array_Length` _returnvalue)) true true (struct :`R` 1.0 :`G` 0.002278 :`A` 1.0) 15.0))

(fn `UserConstructionScript`)