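; Screenshot-sharing test Blueprint that, on R, captures the game screen and shares it to Twitter as an Imgur link.
; It deletes the previous HighResShot file, captures a new one, waits a few frames, then POSTs the binary to a hard-coded server, substituting a static PNG in editor.
; The response is parsed into an Imgur URL for the launched Twitter link.
; Other keys quit, print editor status or debug-upload from the screenshot folder.
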(event `self.ReceiveBeginPlay`
  (`self.EnableInput` (`GameplayStatics.GetPlayerController` 0)))

(event `Key|R`
  (params (Key :type "Key Structure"))
  (:`Pressed`
    (`self.CaptureAndShare`)))

(event `Key|Escape`
  (params (Key :type "Key Structure"))
  (:`Pressed`
    (`KismetSystemLibrary.QuitGame` null "Quit")))

(event `Key|C`
  (params (Key :type "Key Structure"))
  (:`Pressed`
    (`KismetSystemLibrary.PrintString` (`KismetStringLibrary.Concat_StrStr` "With editor: " (`KismetStringLibrary.Conv_BoolToString` (`LowEntryExtendedStandardLibrary.WithEditor`))))))

(event `CaptureAndShare`
  (`self.DeleteLastScreenshot`)
  (`self.CaptureImage` "0.5")
  (`LowEntryExtendedStandardLibrary.DelayFrames` 5)
  (`self.UploadToServer`))

(event `DeleteLastScreenshot`
  (`LowEntryFileManagerFile.Delete` (`LowEntryFileManagerDirectory.GetFile` (`LowEntryFileManagerLibrary.GetDirectory` "../../Saved/Screenshots/WindowsNoEditor/") "HighresScreenshot00000.png")))

(event `CaptureImage`
  (params (Scale :type String :default "0.5"))
  ;[1 1 1] Scale 1 for player screen size, 0.5 for half, 2 for double
  (`KismetSystemLibrary.ExecuteConsoleCommand` (`KismetStringLibrary.Concat_StrStr` "HighResShot " Scale) null))

(event `UploadToServer`
  (bind _returnvalue (`LowEntryFileManagerFile.GetData` (select `bool` (`LowEntryExtendedStandardLibrary.WithEditor`) :`false` (`LowEntryFileManagerDirectory.GetFile` (`LowEntryFileManagerLibrary.GetDirectory` "../../Saved/Screenshots/WindowsNoEditor/") "HighresScreenshot00000.png") :`true` (`LowEntryFileManagerDirectory.GetFile` (`LowEntryFileManagerLibrary.GetRoot`) "4.2.png"))))
  (`KismetSystemLibrary.PrintString` (`KismetStringLibrary.Concat_StrStr` "File size: " (`KismetStringLibrary.Conv_IntToString` (`KismetArrayLibrary.Array_Length` _returnvalue))) true true (struct :`R` 1.0 :`B` 0.419183 :`A` 1.0) 5.0)
  (bind _output_get (set `self.Request` (`VaRestRequestJSON.ConstructRequestExt` "POST" "binary")))
  (`VaRestRequestJSON.SetBinaryRequestContent` _output_get _returnvalue)
  (add `VaRestRequestJSON.OnRequestComplete` _output_get (delegate `Success`) :!label _label)
  ;[1 0 0.1534] server URL
  (`VaRestRequestJSON.ProcessURL` _output_get "http://51.15.205.111:6699/image/"))

(event `Success`
  (params (Request :type "VaRestRequestJSON Object Reference"))
  (bind _returnvalue (`VaRestRequestJSON.GetResponseContentAsString` Request true))
  (`KismetSystemLibrary.PrintString` (`KismetStringLibrary.Concat_StrStr` "Success: " _returnvalue))
  (`KismetSystemLibrary.LaunchURL` (`KismetStringLibrary.Concat_StrStr` (`self.StaticTwitterURL`) "Hello, this is a test " (`KismetStringLibrary.Concat_StrStr` "https://imgur.com/" (`KismetStringLibrary.Split` (`KismetStringLibrary.Split` (`.RightS` (`KismetStringLibrary.Split` _returnvalue "/" "IgnoreCase" "FromEnd")) "\"") ".")))))

(event `Key|T`
  (params (Key :type "Key Structure"))
  ;[1 1 1] Debug
  (:`Pressed`
    (`KismetSystemLibrary.PrintString` "LOOP MODE")
    (for _array_element (`LowEntryFileManagerDirectory.GetFiles` (`LowEntryFileManagerLibrary.GetDirectory` "../../Saved/Screenshots/WindowsNoEditor/"))
      (`KismetSystemLibrary.PrintString` (`LowEntryFileManagerFile.GetName` _array_element))
      (`/Engine/EditorBlueprintResources/StandardMacros.DoOnce` false :!label _label_2
        (:`Completed`
          (bind _output_get (set `self.Request` (`VaRestRequestJSON.ConstructRequestExt` "POST" "binary")))
          (bind _returnvalue (`LowEntryFileManagerFile.GetData` _array_element))
          (`VaRestRequestJSON.SetBinaryRequestContent` _output_get _returnvalue)
          (`KismetSystemLibrary.PrintString` (`KismetStringLibrary.Concat_StrStr` "File size: " (`KismetStringLibrary.Conv_IntToString` (`KismetArrayLibrary.Array_Length` _returnvalue))) true true (struct :`R` 1.0 :`B` 0.419183 :`A` 1.0) 5.0)
          (goto _label))))
    (goto _label_2 :!via `Reset`)))

(fn `UserConstructionScript`)